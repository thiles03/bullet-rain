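; Survival game mode that keeps the world stocked with up to 100 enemies and provides random pickup drops.
; BeginPlay gathers spawn points and counts existing enemies; each Tick below the cap spawns one random minion type at a random point.
; DecrementEnemies lowers the running count, freeing room for replacements.
; SpawnRandomPickup places random armour, health or bullet-time pickups at a given transform, with a roll that practically always succeeds.
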(event `self.ReceiveBeginPlay`
  (set `self.Enemies` (`|MakeArray` "/Game/Characters/Blueprints/BP_Minion_Core.BP_Minion_Core_C" "/Game/Characters/Blueprints/BP_Minion_Dawn.BP_Minion_Dawn_C" "/Game/Characters/Blueprints/BP_Minion_Dusk.BP_Minion_Dusk_C" "/Game/Characters/Blueprints/BP_Minion_Prime.BP_Minion_Prime_C" "/Game/Characters/Blueprints/BP_Minion_White.BP_Minion_White_C" :!type "BR_CharacterEnemy Class Reference"))
  (set `self.Pickups` (`|MakeArray` "/Game/Actors/Pickups/BP_Pickup_Armour.BP_Pickup_Armour_C" "/Game/Actors/Pickups/BP_Pickup_Health.BP_Pickup_Health_C" "/Game/Actors/Pickups/BP_Pickup_BulletTime.BP_Pickup_BulletTime_C" :!type "BR_PickUp_Base Class Reference"))
  (bind _outactors (`GameplayStatics.GetAllActorsOfClass` "/Game/Actors/BP_SpawnPoint.BP_SpawnPoint_C"))
  (set `self.SpawnPoints` _outactors)
  (bind _outactors_2 (`GameplayStatics.GetAllActorsOfClass` "/Script/BulletRain.BR_CharacterEnemy"))
  (set `self.WorldEnemies` (`KismetArrayLibrary.Array_Length` _outactors_2)))

(event `self.ReceiveTick`
  (params (DeltaSeconds :type "Float (single-precision)"))
  (bind _spawnpoints (`self.SpawnPoints`))
  (bind _enemies (`self.Enemies`))
  (if (< (`self.WorldEnemies`) 100)
    (`|SpawnActorFromClass` (`|GetArrayItem` _enemies (`KismetMathLibrary.RandomIntegerInRange` 0 (`KismetArrayLibrary.Array_LastIndex` _enemies))) (`self.GetTransform` (`|GetArrayItem` _spawnpoints (`KismetMathLibrary.RandomIntegerInRange` 0 (`KismetArrayLibrary.Array_LastIndex` _spawnpoints)))) "Undefined" "OverrideRootScale" null null)
    (`/Engine/EditorBlueprintResources/StandardMacros.IncrementInt` (`self.WorldEnemies`))))

(fn `DecrementEnemies`
  (`/Engine/EditorBlueprintResources/StandardMacros.DecrementInt` (`self.WorldEnemies`)))

(fn `SpawnRandomPickup`
  (params (SpawnPoint :type "Transform Structure"))
  (bind _pickups (`self.Pickups`))
  (if (< (`KismetMathLibrary.RandomFloatInRange` 0.0 100.0) 100.0)
    (`|SpawnActorFromClass` (`|GetArrayItem` _pickups (`KismetMathLibrary.RandomIntegerInRange` 0 (`KismetArrayLibrary.Array_LastIndex` _pickups))) SpawnPoint "Undefined" "OverrideRootScale" null null)))

(fn `UserConstructionScript`)