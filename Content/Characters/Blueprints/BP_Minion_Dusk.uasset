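; BP_Minion_Dusk is a minion enemy character that reports to the survival game mode.
; It plays a creature sound cue at its location on BeginPlay.
; Its DecrementWorldEnemies and SpawnPickup events cast to BP_GameMode_Survival to lower the enemy count and spawn a random pickup at the minion's transform.
; Nothing in this graph calls those two events, and Tick and overlap are unused.
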(event `self.DecrementWorldEnemies`
  (bind _asbp_game_mode_survival (cast `/Game/GameModes/BP_GameMode_Survival` (`GameplayStatics.GetGameMode`)))
  (`/Game/GameModes/BP_GameMode_Survival.DecrementEnemies` _asbp_game_mode_survival))

(event `self.SpawnPickup`
  (bind _asbp_game_mode_survival (cast `/Game/GameModes/BP_GameMode_Survival` (`GameplayStatics.GetGameMode`)))
  (`/Game/GameModes/BP_GameMode_Survival.SpawnRandomPickup` _asbp_game_mode_survival (`self.GetTransform` self)))

(event `self.ReceiveBeginPlay`
  (`GameplayStatics.PlaySoundAtLocation` "/Game/_Global/Audio/CUEs/Creature/CUE_Creature.CUE_Creature" (`self.K2_GetActorLocation`) (struct) 1.0 1.0 0.0 null null null))

(fn `UserConstructionScript`)